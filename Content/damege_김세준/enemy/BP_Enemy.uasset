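; BP_Enemy is a melee AI enemy with patrol route, speed settings, health bar and ragdoll death.
; BPCDamageSystem handles incoming damage, with its delegates bound to health and death logic.
; Attacks play a montage, while a looping timer sphere-traces between weapon sockets, stopping on a damaging hit that knocks the player back.
; Once hostile, twenty seconds without damage makes it spawn a fresh copy at its origin and destroy itself.
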(event `Damageresponse`
  (params (Damageresponse :type "/Game/damege_김세준/E_DamageResponse Enum" :default "NewEnumerator0") (`대미지` :type "Float (double-precision)") (NewParam :type "Vector Structure") (NewParam2 :type "Rotator Structure") (NewParam3 :type "/Game/damege_김세준/E_damage_type Enum" :default "NewEnumerator0"))
  ;[1 1 1] 대미지 수신 노드
  (set `self.사라지는 카운트 다운` 0.0)
  (switch `/Game/damege_김세준/E_DamageResponse` Damageresponse
    (:`NewEnumerator1`
      (`AISense_Damage.ReportDamageEvent` self (`GameplayStatics.GetPlayerCharacter` 0) 10.0)
      (`KismetSystemLibrary.PrintString` (`|GetEnumeratorNameAsString` Damageresponse))
      (if (not (`self.deathboleon`))
        (bind _output_get (set `self.current Helth` (`KismetMathLibrary.FClamp` (- (`self.current Helth`) `대미지`) 0.0 (`self.max Helth`))))
        (`/Game/damege_김세준/enemy/enemy_Health_bar.Update enenmy Helth Ui` (stale `self.ReceiveBeginPlay` _returnvalue) _output_get (`self.max Helth`))
        (`GameplayStatics.SpawnEmitterAtLocation` "/Game/StarterContent/Particles/P_Explosion.P_Explosion" (`self.K2_GetActorLocation`))
        (if (>= 0.0 (`self.current Helth`))
          (set `self.deathboleon` true)
          (`self.dead`))))))

(event `dead`
  (bind _mesh (`self.Mesh`))
  ;[1 1 1] 몹 사망 이벤트
  (`PrimitiveComponent.SetSimulatePhysics` _mesh true)
  (`PrimitiveComponent.SetCollisionEnabled` _mesh "QueryAndPhysics")
  (`self.DisableInput` (`GameplayStatics.GetPlayerController` 0))
  (set `self.deathboleon` true)
  (`/Engine/EditorBlueprintResources/StandardMacros.DoOnce` false
    (:`Completed`
      (`ActorComponent.K2_DestroyComponent` (`self.enemy HP bar`))
      (`self.K2_DestroyActor`))))

(event `체력충전`
  ;[1 1 1] UI 업데이트
  (bind _output_get (set `self.current Helth` (`self.max Helth`)))
  (`/Game/damege_김세준/enemy/enemy_Health_bar.Update enenmy Helth Ui` (stale `self.ReceiveBeginPlay` _returnvalue) _output_get (`self.max Helth`)))

(event `attack_montage`
  ;[1 1 1] 공격 모션 불러오기
  (set `self.IS ATTACKING` true)
  (`|ExecutionSequence`
    (:`then_1`
      (set `self.Anim Montage` "/Game/added_anim_KSJ/1117Standing_Melee_Attack_Backhand_KSJ_Montage.1117Standing_Melee_Attack_Backhand_KSJ_Montage")
      (`|PlayMontage` (`self.Mesh`) (`self.Anim Montage`)
        (:`OnCompleted`
          _)
        (:`OnInterrupted`
          _))
      (`self.On attack end`)
      (`KismetSystemLibrary.Delay` 2.7)
      (set `self.IS ATTACKING` false))))

(event `self.ReceiveBeginPlay`
  ;[1 1 1] 플레이어 발견시 위젯 생성 후 소멸 카운트다운 개시
  (set `self.소환 위치` (`self.K2_GetActorLocation`))
  (set `self.소환 방향` (`self.K2_GetActorRotation`))
  (bind _returnvalue (`|CreateWidget` "/Game/damege_김세준/enemy/enemy_Health_bar.enemy_Health_bar_C" null self))
  (`WidgetComponent.SetWidget` (`self.enemy HP bar`) _returnvalue)
  (`self.체력충전`))

(event `적대적 행동자`
  ;[1 1 1] 플레이어 발견시 위젯 생성 후 소멸 카운트다운 개시
  (`SceneComponent.SetHiddenInGame` (`self.enemy HP bar`) false false)
  (bind _returnvalue (`KismetSystemLibrary.K2_SetTimerDelegate` (delegate `안때리면 사라진다`) 1.0 true))
  (set `self.소멸 시간` _returnvalue))

(event `안때리면 사라진다`
  ;[1 1 1] 플레이어 발견시 위젯 생성 후 소멸 카운트다운 개시
  (bind _output_get (set `self.사라지는 카운트 다운` (+ (`self.사라지는 카운트 다운`) 1.0)))
  (`KismetSystemLibrary.PrintString` (`KismetStringLibrary.Conv_DoubleToString` _output_get))
  (if (== (`self.사라지는 카운트 다운`) 20.0)
    (`AIBlueprintHelperLibrary.SpawnAIFromClass` "BP_Enemy_C" "/Game/damege_김세준/enemy/AI_Base/BT_enemybase.BT_enemybase" (`self.소환 위치`) (`self.소환 방향`) false null)
    (`KismetSystemLibrary.K2_ClearAndInvalidateTimerHandle` (`self.소멸 시간`))
    (`self.K2_DestroyActor`)))

(event `sword draw`
  ;[1 1 1] 공격 모션 불러오기
  (`SceneComponent.SetHiddenInGame` (`self.무기`) false false)
  (set `self.draw waepon` true))

(event `공격`
  ;[1 1 1] 공격 로직
  (bind _returnvalue (`KismetSystemLibrary.K2_SetTimerDelegate` (delegate `대미지 처리`) 0.1 true))
  (set `self.무기 휘두르기` _returnvalue))

(event `대미지 처리`
  (bind _capsulecomponent (`self.CapsuleComponent`))
  (bind `_무기` (`self.무기`))
  (bind (_returnvalue_x _returnvalue_y _returnvalue_z) (`KismetMathLibrary.BreakVector` (* (`KismetMathLibrary.GetForwardVector` (`SceneComponent.K2_GetComponentRotation` _capsulecomponent)) 1000.0)))
  ;[1 1 1] 공격 로직
  (if (not (`self.deathboleon`))
    (bind (_outhit _returnvalue) (`KismetSystemLibrary.SphereTraceSingle` :`Start` (`SceneComponent.GetSocketLocation` `_무기` "start") :`End` (`SceneComponent.GetSocketLocation` `_무기` "end") :`Radius` 30.0 :`TraceChannel` "TraceTypeQuery1" :`DrawDebugType` "ForDuration" :`DrawTime` 3.0))
    (if _returnvalue
      (bind (_bblockinghit _binitialoverlap _time _distance _location _impactpoint _normal _impactnormal _physmat _hitactor) (`GameplayStatics.BreakHitResult` _outhit))
      (bind (_wasdamaged `_대미지_입력값`) (message `/Game/damege_김세준/BPI_damagable.takedamage` _hitactor (make `/Game/damege_김세준/s_damageinfo` 1.0 "NewEnumerator1" "NewEnumerator1")))
      (if _wasdamaged
        (`KismetSystemLibrary.PrintString` (`KismetStringLibrary.Conv_DoubleToString` `_대미지_입력값`))
        (`GameplayStatics.SpawnEmitterAtLocation` "/Game/StarterContent/Particles/P_Explosion.P_Explosion" _location)
        (`self.다단히트 금지`)
        (bind _asbp_player_ksj (cast `/Game/damege_김세준/Player/BP_player_KSJ` _hitactor))
        (`self.K2_SetActorRotation` _asbp_player_ksj (`KismetMathLibrary.Conv_VectorToRotator` (* (`KismetMathLibrary.GetForwardVector` (`SceneComponent.K2_GetComponentRotation` _capsulecomponent)) -1.0)) false)
        (`self.LaunchCharacter` _asbp_player_ksj (`KismetMathLibrary.MakeVector` _returnvalue_x _returnvalue_y (+ _returnvalue_z 200.0)) false false)))))

(event `다단히트 금지`
  ;[1 1 1] 공격 로직
  (`KismetSystemLibrary.K2_ClearAndInvalidateTimerHandle` (`self.무기 휘두르기`)))

(fn `gatmaxhealth`
  (returns (maxhealth :type "Float (double-precision)"))
  (return (`self.max Helth`)))

(fn `get idial range`
  (returns (`attack radius` :type "Float (double-precision)") (`defend radius` :type "Float (double-precision)"))
  (return 200.0 300.0))

(fn `get patroll route`
  (returns (`patroll route` :type "/Game/damege_김세준/enemy/AI_Base/patrol_rap Object Reference"))
  (return (`self.patrollroute`)))

(fn `getcurrenthealth`
  (returns (health :type "Float (double-precision)"))
  (return (`self.current Helth`)))

(fn `heal`
  (params (amount :type "Float (double-precision)"))
  (returns (newhealth :type "Float (double-precision)"))
  (bind _newhealth (`/Game/damege_김세준/BPC_damageSystem.heal` (`self.BPC_damageSystem`) amount))
  (return _newhealth))

(fn `set movement speed`
  (params (speed :type "/Game/damege_김세준/enemy/AI_Base/Enums/E_movementspeed Enum" :default "NewEnumerator0"))
  (returns (`speed velue` :type "Float (double-precision)"))
  (bind _output_get (set `CharacterMovementComponent.MaxWalkSpeed` (select `/Game/damege_김세준/enemy/AI_Base/Enums/E_movementspeed` speed :`NewEnumerator1` 100.0 :`NewEnumerator2` 300.0 :`NewEnumerator3` 500.0 :!type "Float (single-precision)") (`self.CharacterMovement`)))
  (return _output_get))

(fn `takedamage`
  (params (Damageinfo :type "/Game/damege_김세준/s_damageinfo Structure"))
  (returns (WasDamaged :type Boolean) (`대미지 입력값` :type "Float (double-precision)"))
  (bind (_was_damaged `_대미지_입력값`) (`/Game/damege_김세준/BPC_damageSystem.TakeDamge` (`self.BPC_damageSystem`) Damageinfo (`self.current Helth`) (`self.max Helth`) (`self.deathboleon`)))
  (return _was_damaged `_대미지_입력값`))

(fn `UserConstructionScript`
  (bind _bpc_damagesystem (`self.BPC_damageSystem`))
  (add `/Game/damege_김세준/BPC_damageSystem.Ondeath` _bpc_damagesystem (`|CreateDelegate` :!event `dead`))
  (add `/Game/damege_김세준/BPC_damageSystem.Ondamageresponse` _bpc_damagesystem (`|CreateDelegate` :!event `Damageresponse`)))