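; Stage 2 standby melee mob that takes player hits through BPCDamageSystem, shows a health bar and ragdolls on death.
; Random montages trigger looping sphere traces on left and right sockets, stopped after one hit.
; Special wrench and hammer attacks interrupt and stun it; a timed stun state enables a box that spreads stun on overlap.
; Once hostile, it respawns fresh at its origin after 20 seconds without player hits.
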(event `self.Box.OnComponentBeginOverlap`
  (params (OverlappedComponent :type "PrimitiveComponent Object Reference") (OtherActor :type "Actor Object Reference") (OtherComp :type "PrimitiveComponent Object Reference") (OtherBodyIndex :type Integer) (bFromSweep :type Boolean) (SweepResult :type "HitResult Structure (by ref)"))
  ;[1 1 1] 스턴 로직
  (message `/Game/damege_김세준/BPI_damagable.takedamage` OtherActor (make `/Game/damege_김세준/s_damageinfo` 1.0 "NewEnumerator2" "NewEnumerator3" false false false false (`SceneComponent.K2_GetComponentLocation` (`self.Box`)) (`KismetMathLibrary.Conv_VectorToRotator` (* (`SceneComponent.GetForwardVector` (`self.CapsuleComponent`)) -1.0)))))

(event `스턴`
  ;[1 1 1] 스턴 로직
  (set `PrimitiveComponent.bGenerateOverlapEvents` true (`self.Box`))
  (bind _returnvalue (`KismetSystemLibrary.K2_SetTimerDelegate` (delegate `앞잡 카운트다운`) 1.0 true))
  (set `self.앞잡 타이머` _returnvalue))

(event `Damageresponse`
  (params (Damageresponse :type "/Game/damege_김세준/E_DamageResponse Enum" :default "NewEnumerator0") (`대미지` :type "Float (double-precision)") (NewParam :type "Vector Structure") (NewParam2 :type "Rotator Structure") (NewParam3 :type "/Game/damege_김세준/E_damage_type Enum" :default "NewEnumerator0"))
  (bind (_returnvalue_x _returnvalue_y _returnvalue_z) (`KismetMathLibrary.BreakVector` (* NewParam 1200.0)))
  ;[1 1 1] 피격 판정
  (switch `/Game/damege_김세준/E_damage_type` NewParam3
    (:`NewEnumerator1`
      (set `self.사라지는 카운트 다운` 0.0)
      (switch `/Game/damege_김세준/E_DamageResponse` Damageresponse
        (:`NewEnumerator1`
          (if (`self.IS ATTACKING`)
            (bind _returnvalue (`GameplayStatics.GetActorOfClass` "/Game/damege_김세준/Player/BP_player_KSJ.BP_player_KSJ_C"))
            (`/Game/damege_김세준/Player/BP_player_KSJ.필살기 게이지 충전_Event` _returnvalue))
          (`AISense_Hearing.ReportNoiseEvent` (`self.K2_GetActorLocation`) 30.0 (`GameplayStatics.GetPlayerCharacter` 0) 50.0 :!label _label)
          (`AISense_Damage.ReportDamageEvent` self (`GameplayStatics.GetPlayerCharacter` 0) 10.0)
          (`KismetSystemLibrary.PrintString` (`|GetEnumeratorNameAsString` Damageresponse))
          (if (not (`self.deathboleon`))
            (`GameplayStatics.PlaySoundAtLocation` "/Game/Sound_AHJ/Cue/Monster/GetHit/Cue_Monster_GetHit_Normal_SFX.Cue_Monster_GetHit_Normal_SFX" (0.0 0.0 0.0) (struct) 1.0 1.0 0.0 null null null null)
            (bind _output_get (set `self.current Helth` (`KismetMathLibrary.FClamp` (- (`self.current Helth`) `대미지`) 0.0 (`self.max Helth`))))
            (`/Game/damege_김세준/enemy/enemy_Health_bar.Update enenmy Helth Ui` (stale `self.ReceiveBeginPlay` _returnvalue) _output_get (`self.max Helth`))
            (`GameplayStatics.SpawnEmitterAtLocation` "/Game/StarterContent/Particles/P_Explosion.P_Explosion" (`self.K2_GetActorLocation`))
            (if (>= 0.0 (`self.current Helth`))
              (set `self.deathboleon` true)
              (`self.dead`))))
        (:`NewEnumerator2`
          (`KismetSystemLibrary.K2_ClearAndInvalidateTimerHandle` (`self.앞잡 타이머`))
          (set `self.앞잡 계산기` 0.0))
        (:`NewEnumerator3`
          (goto _label))
        (:`NewEnumerator4`
          (set `self.넉백` true)
          (`self.LaunchCharacter` (`KismetMathLibrary.MakeVector` _returnvalue_x _returnvalue_y _returnvalue_z))
          (`KismetSystemLibrary.Delay` 2.0)
          (set `self.IS stun` false)
          (`self.스턴해제`)
          (`self.On attack end`)
          (set `PrimitiveComponent.bGenerateOverlapEvents` false (`self.Box`))
          (set `self.넉백` false))))
    (:`NewEnumerator3`
      (set `self.IS ATTACKING` false)
      (`self.StopAnimMontage` (`self.공격모션`))
      (set `self.IS stun` true)
      (`GameplayStatics.PlaySoundAtLocation` "/Game/Sound_AHJ/Cue/Monster/GetHit/Cue_Monster_GetHit_Groggy_SFX.Cue_Monster_GetHit_Groggy_SFX" (0.0 0.0 0.0) (struct) 1.0 1.0 0.0 null null null null))
    (:`NewEnumerator4`
      (set `self.IS ATTACKING` false)
      (`self.StopAnimMontage` (`self.공격모션`))
      (set `self.IS stun` true)
      (goto _label))))

(event `앞잡 카운트다운`
  ;[1 1 1] 스턴 로직
  (bind _output_get (set `self.앞잡 계산기` (+ (`self.앞잡 계산기`) 1.0)))
  (if (== _output_get 3.0)
    (`self.스턴해제`)
    (`self.On attack end`)
    (set `self.IS stun` false)
    (set `PrimitiveComponent.bGenerateOverlapEvents` false (`self.Box`))))

(event `attack_montage`
  (bind _returnvalue (`KismetMathLibrary.RandomInteger` (`self.공격 빈도`)))
  ;[1 1 1] 공격 모션 불러오기
  (set `self.IS ATTACKING` true)
  (if (`self.deathboleon`)
    (`self.On attack end`)
    (elif (> _returnvalue 69)
      (set `self.공격모션` "/Game/damege_김세준/enemy/2st_Mobs/anim_base/240106_A_attack_01_KSJ_Montage.240106_A_attack_01_KSJ_Montage")
      (`|PlayMontage` (`self.Mesh`) (`self.공격모션`) :!label _label_2
        (:`OnCompleted`
          (`self.On attack end` :!label _label_3)
          (set `self.IS ATTACKING` false)
          (`KismetSystemLibrary.K2_ClearAndInvalidateTimerHandle` (`self.무기 휘두르기`) :!label _label_4)
          (bind _returnvalue_2 (`GameplayStatics.GetActorOfClass` "/Game/damege_김세준/Player/BP_player_KSJ.BP_player_KSJ_C"))
          (if (not (`SceneComponent.bHiddenInGame` (`/Game/damege_김세준/Player/BP_player_KSJ.TextRender` _returnvalue_2)))
            (`/Game/damege_김세준/Player/BP_player_KSJ.알림 제거_Event` _returnvalue_2)))
        (:`OnInterrupted`
          (goto _label_3))
        (:`OnNotifyBegin`
          (`self.공격` :!label _label_5))
        (:`OnNotifyEnd`
          (goto _label_4)))
      (elif (> _returnvalue 39)
        (set `self.공격모션` "/Game/damege_김세준/enemy/2st_Mobs/anim_base/240106_A_attack_01_KSJ_Montage.240106_A_attack_01_KSJ_Montage")
        (`|PlayMontage` (`self.Mesh`) (`self.공격모션`)
          (:`OnCompleted`
            (set `self.공격모션` "/Game/damege_김세준/enemy/2st_Mobs/anim_base/240106_A_attack_02_KSJ_Montage.240106_A_attack_02_KSJ_Montage")
            (goto _label_2))
          (:`OnInterrupted`
            (goto _label_3))
          (:`OnNotifyBegin`
            (goto _label_5))
          (:`OnNotifyEnd`
            (goto _label_4)))
        (elif (> _returnvalue 9)
          (set `self.공격모션` "/Game/damege_김세준/enemy/2st_Mobs/anim_base/240106_A_attack_03_KSJ_Montage.240106_A_attack_03_KSJ_Montage")
          (goto _label_2)
          (else
            (set `self.공격모션` "/Game/damege_김세준/enemy/2st_Mobs/anim_base/240106_A_attack_run_KSJ_Montage.240106_A_attack_run_KSJ_Montage")
            (goto _label_2)))))))

(event `체력충전`
  ;[1 1 1] UI 업데이트
  (bind _output_get (set `self.current Helth` (`self.max Helth`)))
  (`/Game/damege_김세준/enemy/enemy_Health_bar.Update enenmy Helth Ui` (stale `self.ReceiveBeginPlay` _returnvalue) _output_get (`self.max Helth`)))

(event `self.ReceiveBeginPlay`
  ;[1 1 1] 플레이어 발견시 위젯 생성 후 소멸 카운트다운 개시
  (set `self.소환 위치` (`self.K2_GetActorLocation`))
  (set `self.소환 방향` (`self.K2_GetActorRotation`))
  (bind _returnvalue (`|CreateWidget` "/Game/damege_김세준/enemy/enemy_Health_bar.enemy_Health_bar_C" null self))
  (`WidgetComponent.SetWidget` (`self.enemy HP bar`) _returnvalue)
  (`self.체력충전`))

(event `적대적 행동자`
  ;[1 1 1] 플레이어 발견시 위젯 생성 후 소멸 카운트다운 개시
  (set `self.draw waepon` true)
  (`SceneComponent.SetHiddenInGame` (`self.enemy HP bar`) false false)
  (bind _returnvalue (`KismetSystemLibrary.K2_SetTimerDelegate` (delegate `안때리면 사라진다`) 1.0 true))
  (set `self.소멸 시간` _returnvalue))

(event `안때리면 사라진다`
  ;[1 1 1] 플레이어 발견시 위젯 생성 후 소멸 카운트다운 개시
  (bind _output_get (set `self.사라지는 카운트 다운` (+ (`self.사라지는 카운트 다운`) 1.0)))
  (`KismetSystemLibrary.PrintString` (`KismetStringLibrary.Conv_DoubleToString` _output_get))
  ;;[1 1 1] 재소환시 인공지능 넣기
  (if (== (`self.사라지는 카운트 다운`) 20.0)
    (`AIBlueprintHelperLibrary.SpawnAIFromClass` "BP_2st_Mob_대기_C" "/Game/damege_김세준/enemy/2st_Mobs/2st_mob_type_대기/BT_2st_mob_대기.BT_2st_mob_대기" (`self.소환 위치`) (`self.소환 방향`) false null)
    (`KismetSystemLibrary.K2_ClearAndInvalidateTimerHandle` (`self.소멸 시간`))
    (`self.K2_DestroyActor`)))

(event `dead`
  (bind _mesh (`self.Mesh`))
  ;[1 1 1] 몹 사망 이벤트
  (`PrimitiveComponent.SetSimulatePhysics` _mesh true)
  (`PrimitiveComponent.SetCollisionEnabled` _mesh "QueryAndPhysics")
  (set `self.deathboleon` true)
  (`/Engine/EditorBlueprintResources/StandardMacros.DoOnce` false
    (:`Completed`
      (`ActorComponent.K2_DestroyComponent` (`self.enemy HP bar`))
      (`KismetSystemLibrary.K2_ClearAndInvalidateTimerHandle` (`self.소멸 시간`)))))

(event `공격`
  ;[1 1 1] 공격 로직
  (bind _returnvalue (`KismetSystemLibrary.K2_SetTimerDelegate` (delegate `대미지 처리`) 0.01 true))
  (set `self.무기 휘두르기` _returnvalue)
  (bind _returnvalue_2 (`GameplayStatics.GetActorOfClass` "/Game/damege_김세준/Player/BP_player_KSJ.BP_player_KSJ_C"))
  (if (`SceneComponent.bHiddenInGame` (`/Game/damege_김세준/Player/BP_player_KSJ.TextRender` _returnvalue_2))
    (`/Game/damege_김세준/Player/BP_player_KSJ.딜레이캐치 알림_Event` _returnvalue_2)))

(event `대미지 처리`
  (bind _mesh (`self.Mesh`))
  (bind _mesh_2 (`self.Mesh`))
  ;[1 1 1] 공격 로직
  (if (not (`self.deathboleon`))
    (`|ExecutionSequence`
      (:`then_0`
        (bind (_outhit _returnvalue) (`KismetSystemLibrary.SphereTraceSingle` :`Start` (`SceneComponent.GetSocketLocation` _mesh "R_start") :`End` (`SceneComponent.GetSocketLocation` _mesh "R_end") :`Radius` 30.0 :`TraceChannel` "TraceTypeQuery1" :`DrawTime` 3.0))
        (if _returnvalue
          (bind (_bblockinghit _binitialoverlap _time _distance _location _impactpoint _normal _impactnormal _physmat _hitactor) (`GameplayStatics.BreakHitResult` _outhit))
          (bind (_wasdamaged `_대미지_입력값`) (message `/Game/damege_김세준/BPI_damagable.takedamage` _hitactor (make `/Game/damege_김세준/s_damageinfo` 1.0 "NewEnumerator2" "NewEnumerator1" false false false false (`KismetMathLibrary.GetForwardVector` (`SceneComponent.K2_GetComponentRotation` (`self.CapsuleComponent`))))))
          (if _wasdamaged
            (`KismetSystemLibrary.PrintString` (`KismetStringLibrary.Conv_DoubleToString` `_대미지_입력값`))
            (`GameplayStatics.SpawnEmitterAtLocation` "/Game/StarterContent/Particles/P_Explosion.P_Explosion" _location)
            (`self.다단히트 금지` :!label _label_6))))
      (:`then_1`
        (bind (_outhit_2 _returnvalue_2) (`KismetSystemLibrary.SphereTraceSingle` :`Start` (`SceneComponent.GetSocketLocation` _mesh_2 "L_start") :`End` (`SceneComponent.GetSocketLocation` _mesh_2 "L_end") :`Radius` 30.0 :`TraceChannel` "TraceTypeQuery1" :`DrawTime` 3.0))
        (if _returnvalue_2
          (bind (_bblockinghit_2 _binitialoverlap_2 _time_2 _distance_2 _location_2 _impactpoint_2 _normal_2 _impactnormal_2 _physmat_2 _hitactor_2) (`GameplayStatics.BreakHitResult` _outhit_2))
          (bind (_wasdamaged_2 `_대미지_입력값_2`) (message `/Game/damege_김세준/BPI_damagable.takedamage` _hitactor_2 (make `/Game/damege_김세준/s_damageinfo` 1.0 "NewEnumerator2" "NewEnumerator1" false false false false (`KismetMathLibrary.GetForwardVector` (`SceneComponent.K2_GetComponentRotation` (`self.CapsuleComponent`))))))
          (if _wasdamaged_2
            (`KismetSystemLibrary.PrintString` (`KismetStringLibrary.Conv_DoubleToString` `_대미지_입력값_2`))
            (`GameplayStatics.SpawnEmitterAtLocation` "/Game/StarterContent/Particles/P_Explosion.P_Explosion" _location_2)
            (goto _label_6)))))))

(event `다단히트 금지`
  ;[1 1 1] 공격 로직
  (`KismetSystemLibrary.K2_ClearAndInvalidateTimerHandle` (`self.무기 휘두르기`)))

(fn `gatmaxhealth`
  (returns (maxhealth :type "Float (double-precision)"))
  (return (`self.max Helth`)))

(fn `get idial range`
  (returns (`attack radius` :type "Float (double-precision)") (`defend radius` :type "Float (double-precision)"))
  (return 200.0 300.0))

(fn `get patroll route`
  (returns (`patroll route` :type "/Game/damege_김세준/enemy/AI_Base/patrol_rap Object Reference"))
  (return (`self.patrollroute`)))

(fn `getcurrenthealth`
  (returns (health :type "Float (double-precision)"))
  (return (`self.current Helth`)))

(fn `heal`
  (params (amount :type "Float (double-precision)"))
  (returns (newhealth :type "Float (double-precision)"))
  (bind _newhealth (`/Game/damege_김세준/BPC_damageSystem.heal` (`self.BPC_damageSystem`) amount))
  (return _newhealth))

(fn `set movement speed`
  (params (speed :type "/Game/damege_김세준/enemy/AI_Base/Enums/E_movementspeed Enum" :default "NewEnumerator0"))
  (returns (`speed velue` :type "Float (double-precision)"))
  (bind _output_get (set `CharacterMovementComponent.MaxWalkSpeed` (select `/Game/damege_김세준/enemy/AI_Base/Enums/E_movementspeed` speed :`NewEnumerator1` 100.0 :`NewEnumerator2` 300.0 :`NewEnumerator3` 500.0 :!type "Float (single-precision)") (`self.CharacterMovement`)))
  (return _output_get))

(fn `takedamage`
  (params (Damageinfo :type "/Game/damege_김세준/s_damageinfo Structure"))
  (returns (WasDamaged :type Boolean) (`대미지 입력값` :type "Float (double-precision)"))
  (bind (_was_damaged `_대미지_입력값`) (`/Game/damege_김세준/BPC_damageSystem.TakeDamge` (`self.BPC_damageSystem`) Damageinfo (`self.current Helth`) (`self.max Helth`) (`self.deathboleon`)))
  (return _was_damaged `_대미지_입력값`))

(fn `UserConstructionScript`
  (bind _bpc_damagesystem (`self.BPC_damageSystem`))
  (add `/Game/damege_김세준/BPC_damageSystem.Ondeath` _bpc_damagesystem (`|CreateDelegate` :!event `dead`))
  (add `/Game/damege_김세준/BPC_damageSystem.Ondamageresponse` _bpc_damagesystem (`|CreateDelegate` :!event `Damageresponse`)))