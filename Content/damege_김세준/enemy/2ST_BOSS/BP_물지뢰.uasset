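; Water mine hazard for the Stage 2 boss: ten spheres that appear as waterfall effects and explode on player touch or timeout.
; BeginPlay reveals them one by one, enabling overlaps (except Sphere4), while a delayed parallel chain fires each timeout event before destroying the actor.
; Overlap and timeout share a DoOnce per sphere that plays sound and explosion, sends damage to OtherActor and removes the waterfall.
; Sphere2 compares OtherComp, not OtherActor, to the player.
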(event `self.ReceiveBeginPlay`
  (bind _sphere_1 (`self.Sphere 1`))
  (bind _sphere_2 (`self.Sphere 2`))
  (bind _sphere_3 (`self.Sphere 3`))
  (bind _sphere_5 (`self.Sphere 5`))
  (bind _sphere_6 (`self.Sphere 6`))
  (bind _sphere_7 (`self.Sphere 7`))
  (bind _sphere_8 (`self.Sphere 8`))
  (bind _sphere_9 (`self.Sphere 9`))
  (bind _sphere_10 (`self.Sphere 10`))
  (`|ExecutionSequence`
    (:`then_0`
      (`/Engine/EditorBlueprintResources/StandardMacros.DoOnce` false
        (:`Completed`
          (`KismetSystemLibrary.Delay` 10.0)
          (`self.시간제한 1`)
          (`KismetSystemLibrary.Delay` (`self.Duration`))
          (`self.시간제한 2`)
          (`KismetSystemLibrary.Delay` (`self.Duration`))
          (`self.시간제한 3`)
          (`KismetSystemLibrary.Delay` (`self.Duration`))
          (`self.시간제한 4`)
          (`KismetSystemLibrary.Delay` (`self.Duration`))
          (`self.시간제한 5`)
          (`KismetSystemLibrary.Delay` (`self.Duration`))
          (`self.시간제한 6`)
          (`KismetSystemLibrary.Delay` (`self.Duration`))
          (`self.시간제한 7`)
          (`KismetSystemLibrary.Delay` (`self.Duration`))
          (`self.시간제한 8`)
          (`KismetSystemLibrary.Delay` (`self.Duration`))
          (`self.시간제한 9`)
          (`KismetSystemLibrary.Delay` (`self.Duration`))
          (`self.시간제한 10`)
          (`self.K2_DestroyActor`))))
    (:`then_1`
      (set `PrimitiveComponent.bGenerateOverlapEvents` true _sphere_1)
      (bind _returnvalue (`GameplayStatics.SpawnEmitterAtLocation` "/Game/Sewerage/Particles/PS_WaterFall5.PS_WaterFall5" (`SceneComponent.K2_GetComponentLocation` _sphere_1) (struct :`Pitch` 90.0)))
      (set `self.NewVar_1` _returnvalue)
      (`KismetSystemLibrary.Delay` (`self.Duration`))
      (set `PrimitiveComponent.bGenerateOverlapEvents` true _sphere_2)
      (bind _returnvalue_2 (`GameplayStatics.SpawnEmitterAtLocation` "/Game/Sewerage/Particles/PS_WaterFall5.PS_WaterFall5" (`SceneComponent.K2_GetComponentLocation` _sphere_2) (struct :`Pitch` 90.0)))
      (set `self.NewVar_2` _returnvalue_2)
      (`KismetSystemLibrary.Delay` (`self.Duration`))
      (set `PrimitiveComponent.bGenerateOverlapEvents` true _sphere_3)
      (bind _returnvalue_3 (`GameplayStatics.SpawnEmitterAtLocation` "/Game/Sewerage/Particles/PS_WaterFall5.PS_WaterFall5" (`SceneComponent.K2_GetComponentLocation` _sphere_3) (struct :`Pitch` 90.0)))
      (set `self.NewVar_3` _returnvalue_3)
      (`KismetSystemLibrary.Delay` (`self.Duration`))
      (bind _returnvalue_4 (`GameplayStatics.SpawnEmitterAtLocation` "/Game/Sewerage/Particles/PS_WaterFall5.PS_WaterFall5" (`SceneComponent.K2_GetComponentLocation` (`self.Sphere 4`)) (struct :`Pitch` 90.0)))
      (set `self.NewVar_4` _returnvalue_4)
      (`KismetSystemLibrary.Delay` (`self.Duration`))
      (set `PrimitiveComponent.bGenerateOverlapEvents` true _sphere_5)
      (bind _returnvalue_5 (`GameplayStatics.SpawnEmitterAtLocation` "/Game/Sewerage/Particles/PS_WaterFall5.PS_WaterFall5" (`SceneComponent.K2_GetComponentLocation` _sphere_5) (struct :`Pitch` 90.0)))
      (set `self.NewVar_5` _returnvalue_5)
      (`KismetSystemLibrary.Delay` (`self.Duration`))
      (set `PrimitiveComponent.bGenerateOverlapEvents` true _sphere_6)
      (bind _returnvalue_6 (`GameplayStatics.SpawnEmitterAtLocation` "/Game/Sewerage/Particles/PS_WaterFall5.PS_WaterFall5" (`SceneComponent.K2_GetComponentLocation` _sphere_6) (struct :`Pitch` 90.0)))
      (set `self.NewVar_6` _returnvalue_6)
      (`KismetSystemLibrary.Delay` (`self.Duration`))
      (set `PrimitiveComponent.bGenerateOverlapEvents` true _sphere_7)
      (bind _returnvalue_7 (`GameplayStatics.SpawnEmitterAtLocation` "/Game/Sewerage/Particles/PS_WaterFall5.PS_WaterFall5" (`SceneComponent.K2_GetComponentLocation` _sphere_7) (struct :`Pitch` 90.0)))
      (set `self.NewVar_7` _returnvalue_7)
      (`KismetSystemLibrary.Delay` (`self.Duration`))
      (set `PrimitiveComponent.bGenerateOverlapEvents` true _sphere_8)
      (bind _returnvalue_8 (`GameplayStatics.SpawnEmitterAtLocation` "/Game/Sewerage/Particles/PS_WaterFall5.PS_WaterFall5" (`SceneComponent.K2_GetComponentLocation` _sphere_8) (struct :`Pitch` 90.0)))
      (set `self.NewVar_8` _returnvalue_8)
      (`KismetSystemLibrary.Delay` (`self.Duration`))
      (set `PrimitiveComponent.bGenerateOverlapEvents` true _sphere_9)
      (bind _returnvalue_9 (`GameplayStatics.SpawnEmitterAtLocation` "/Game/Sewerage/Particles/PS_WaterFall5.PS_WaterFall5" (`SceneComponent.K2_GetComponentLocation` _sphere_9) (struct :`Pitch` 90.0)))
      (set `self.NewVar_9` _returnvalue_9)
      (`KismetSystemLibrary.Delay` (`self.Duration`))
      (set `PrimitiveComponent.bGenerateOverlapEvents` true _sphere_10)
      (bind _returnvalue_10 (`GameplayStatics.SpawnEmitterAtLocation` "/Game/Sewerage/Particles/PS_WaterFall5.PS_WaterFall5" (`SceneComponent.K2_GetComponentLocation` _sphere_10) (struct :`Pitch` 90.0)))
      (set `self.NewVar_10` _returnvalue_10)
      (`KismetSystemLibrary.Delay` (`self.Duration`)))))

(event `시간제한 1`
  (bind (_returnvalue_x _returnvalue_y _returnvalue_z) (`KismetMathLibrary.BreakVector` (`KismetMathLibrary.GetForwardVector` (`SceneComponent.K2_GetComponentRotation` (`self.RootComponent`)))))
  (`/Engine/EditorBlueprintResources/StandardMacros.DoOnce` false :!label _label
    (:`Completed`
      (`|ExecutionSequence`
        (:`then_0`
          (`GameplayStatics.SpawnSoundAtLocation` "/Game/Sound_AHJ/Cue/Monster/Phase/Cue_Monster_Stage_02_Phase_02_SFX.Cue_Monster_Stage_02_Phase_02_SFX" (0.0 0.0 0.0) (struct) 1.0 1.0 0.0 null null))
        (:`then_1`
          (`GameplayStatics.SpawnEmitterAtLocation` "/Game/StarterContent/Particles/P_Explosion1.P_Explosion1" (`SceneComponent.K2_GetComponentLocation` (`self.Sphere 1`)) (struct) (5.0 5.0 5.0))
          (message `/Game/damege_김세준/BPI_damagable.takedamage` (stale `self.Sphere 1.OnComponentBeginOverlap` OtherActor) (make `/Game/damege_김세준/s_damageinfo` 1.0 "NewEnumerator2" "NewEnumerator1" false false false false (`KismetMathLibrary.MakeVector` (* _returnvalue_x -1.0) (* _returnvalue_y -1.0) _returnvalue_z)))
          (`ActorComponent.K2_DestroyComponent` (`self.NewVar_1`)))))))

(event `시간제한 6`
  (`/Engine/EditorBlueprintResources/StandardMacros.DoOnce` false :!label _label_2
    (:`Completed`
      (`|ExecutionSequence`
        (:`then_0`
          (`GameplayStatics.SpawnSoundAtLocation` "/Game/Sound_AHJ/Cue/Monster/Phase/Cue_Monster_Stage_02_Phase_02_SFX.Cue_Monster_Stage_02_Phase_02_SFX" (0.0 0.0 0.0) (struct) 1.0 1.0 0.0 null null))
        (:`then_1`
          (`GameplayStatics.SpawnEmitterAtLocation` "/Game/StarterContent/Particles/P_Explosion1.P_Explosion1" (`SceneComponent.K2_GetComponentLocation` (`self.Sphere 6`)) (struct) (5.0 5.0 5.0))
          (bind (_returnvalue_x _returnvalue_y _returnvalue_z) (`KismetMathLibrary.BreakVector` (`KismetMathLibrary.GetForwardVector` (`SceneComponent.K2_GetComponentRotation` (`Actor.RootComponent` (stale `self.Sphere 6.OnComponentBeginOverlap` OtherActor))))))
          (message `/Game/damege_김세준/BPI_damagable.takedamage` (stale `self.Sphere 6.OnComponentBeginOverlap` OtherActor) (make `/Game/damege_김세준/s_damageinfo` 1.0 "NewEnumerator2" "NewEnumerator1" false false false false (`KismetMathLibrary.MakeVector` (* _returnvalue_x -1.0) (* _returnvalue_y -1.0) _returnvalue_z)))
          (`ActorComponent.K2_DestroyComponent` (`self.NewVar_6`)))))))

(event `self.Sphere 6.OnComponentBeginOverlap`
  (params (OverlappedComponent :type "PrimitiveComponent Object Reference") (OtherActor :type "Actor Object Reference") (OtherComp :type "PrimitiveComponent Object Reference") (OtherBodyIndex :type Integer) (bFromSweep :type Boolean) (SweepResult :type "HitResult Structure (by ref)"))
  (if (== OtherActor (`GameplayStatics.GetPlayerCharacter` 0))
    (goto _label_2)))

(event `self.Sphere 1.OnComponentBeginOverlap`
  (params (OverlappedComponent :type "PrimitiveComponent Object Reference") (OtherActor :type "Actor Object Reference") (OtherComp :type "PrimitiveComponent Object Reference") (OtherBodyIndex :type Integer) (bFromSweep :type Boolean) (SweepResult :type "HitResult Structure (by ref)"))
  (if (== OtherActor (`GameplayStatics.GetPlayerCharacter` 0))
    (goto _label)))

(event `시간제한 7`
  (`/Engine/EditorBlueprintResources/StandardMacros.DoOnce` false :!label _label_3
    (:`Completed`
      (`|ExecutionSequence`
        (:`then_0`
          (`GameplayStatics.SpawnSoundAtLocation` "/Game/Sound_AHJ/Cue/Monster/Phase/Cue_Monster_Stage_02_Phase_02_SFX.Cue_Monster_Stage_02_Phase_02_SFX" (0.0 0.0 0.0) (struct) 1.0 1.0 0.0 null null))
        (:`then_1`
          (`GameplayStatics.SpawnEmitterAtLocation` "/Game/StarterContent/Particles/P_Explosion1.P_Explosion1" (`SceneComponent.K2_GetComponentLocation` (`self.Sphere 7`)) (struct) (5.0 5.0 5.0))
          (bind (_returnvalue_x _returnvalue_y _returnvalue_z) (`KismetMathLibrary.BreakVector` (`KismetMathLibrary.GetForwardVector` (`SceneComponent.K2_GetComponentRotation` (`Actor.RootComponent` (stale `self.Sphere 7.OnComponentBeginOverlap` OtherActor))))))
          (message `/Game/damege_김세준/BPI_damagable.takedamage` (stale `self.Sphere 7.OnComponentBeginOverlap` OtherActor) (make `/Game/damege_김세준/s_damageinfo` 1.0 "NewEnumerator2" "NewEnumerator1" false false false false (`KismetMathLibrary.MakeVector` (* _returnvalue_x -1.0) (* _returnvalue_y -1.0) _returnvalue_z)))
          (`ActorComponent.K2_DestroyComponent` (`self.NewVar_7`)))))))

(event `시간제한 2`
  (`/Engine/EditorBlueprintResources/StandardMacros.DoOnce` false :!label _label_4
    (:`Completed`
      (`|ExecutionSequence`
        (:`then_0`
          (`GameplayStatics.SpawnSoundAtLocation` "/Game/Sound_AHJ/Cue/Monster/Phase/Cue_Monster_Stage_02_Phase_02_SFX.Cue_Monster_Stage_02_Phase_02_SFX" (0.0 0.0 0.0) (struct) 1.0 1.0 0.0 null null))
        (:`then_1`
          (`GameplayStatics.SpawnEmitterAtLocation` "/Game/StarterContent/Particles/P_Explosion1.P_Explosion1" (`SceneComponent.K2_GetComponentLocation` (`self.Sphere 2`)) (struct) (5.0 5.0 5.0))
          (bind (_returnvalue_x _returnvalue_y _returnvalue_z) (`KismetMathLibrary.BreakVector` (`KismetMathLibrary.GetForwardVector` (`SceneComponent.K2_GetComponentRotation` (`Actor.RootComponent` (stale `self.Sphere 2.OnComponentBeginOverlap` OtherActor))))))
          (message `/Game/damege_김세준/BPI_damagable.takedamage` (stale `self.Sphere 2.OnComponentBeginOverlap` OtherActor) (make `/Game/damege_김세준/s_damageinfo` 1.0 "NewEnumerator2" "NewEnumerator1" false false false false (`KismetMathLibrary.MakeVector` (* _returnvalue_x -1.0) (* _returnvalue_y -1.0) _returnvalue_z)))
          (`ActorComponent.K2_DestroyComponent` (`self.NewVar_2`)))))))

(event `self.Sphere 7.OnComponentBeginOverlap`
  (params (OverlappedComponent :type "PrimitiveComponent Object Reference") (OtherActor :type "Actor Object Reference") (OtherComp :type "PrimitiveComponent Object Reference") (OtherBodyIndex :type Integer) (bFromSweep :type Boolean) (SweepResult :type "HitResult Structure (by ref)"))
  (if (== OtherActor (`GameplayStatics.GetPlayerCharacter` 0))
    (goto _label_3)))

(event `self.Sphere 2.OnComponentBeginOverlap`
  (params (OverlappedComponent :type "PrimitiveComponent Object Reference") (OtherActor :type "Actor Object Reference") (OtherComp :type "PrimitiveComponent Object Reference") (OtherBodyIndex :type Integer) (bFromSweep :type Boolean) (SweepResult :type "HitResult Structure (by ref)"))
  (if (== OtherComp (`GameplayStatics.GetPlayerCharacter` 0))
    (goto _label_4)))

(event `시간제한 8`
  (`/Engine/EditorBlueprintResources/StandardMacros.DoOnce` false :!label _label_5
    (:`Completed`
      (`|ExecutionSequence`
        (:`then_0`
          (`GameplayStatics.SpawnSoundAtLocation` "/Game/Sound_AHJ/Cue/Monster/Phase/Cue_Monster_Stage_02_Phase_02_SFX.Cue_Monster_Stage_02_Phase_02_SFX" (0.0 0.0 0.0) (struct) 1.0 1.0 0.0 null null))
        (:`then_1`
          (`GameplayStatics.SpawnEmitterAtLocation` "/Game/StarterContent/Particles/P_Explosion1.P_Explosion1" (`SceneComponent.K2_GetComponentLocation` (`self.Sphere 8`)) (struct) (5.0 5.0 5.0))
          (bind (_returnvalue_x _returnvalue_y _returnvalue_z) (`KismetMathLibrary.BreakVector` (`KismetMathLibrary.GetForwardVector` (`SceneComponent.K2_GetComponentRotation` (`Actor.RootComponent` (stale `self.Sphere 8.OnComponentBeginOverlap` OtherActor))))))
          (message `/Game/damege_김세준/BPI_damagable.takedamage` (stale `self.Sphere 8.OnComponentBeginOverlap` OtherActor) (make `/Game/damege_김세준/s_damageinfo` 1.0 "NewEnumerator2" "NewEnumerator1" false false false false (`KismetMathLibrary.MakeVector` (* _returnvalue_x -1.0) (* _returnvalue_y -1.0) _returnvalue_z)))
          (`ActorComponent.K2_DestroyComponent` (`self.NewVar_8`)))))))

(event `시간제한 3`
  (`/Engine/EditorBlueprintResources/StandardMacros.DoOnce` false :!label _label_6
    (:`Completed`
      (`|ExecutionSequence`
        (:`then_0`
          (`GameplayStatics.SpawnSoundAtLocation` "/Game/Sound_AHJ/Cue/Monster/Phase/Cue_Monster_Stage_02_Phase_02_SFX.Cue_Monster_Stage_02_Phase_02_SFX" (0.0 0.0 0.0) (struct) 1.0 1.0 0.0 null null))
        (:`then_1`
          (`GameplayStatics.SpawnEmitterAtLocation` "/Game/StarterContent/Particles/P_Explosion1.P_Explosion1" (`SceneComponent.K2_GetComponentLocation` (`self.Sphere 3`)) (struct) (5.0 5.0 5.0))
          (bind (_returnvalue_x _returnvalue_y _returnvalue_z) (`KismetMathLibrary.BreakVector` (`KismetMathLibrary.GetForwardVector` (`SceneComponent.K2_GetComponentRotation` (`Actor.RootComponent` (stale `self.Sphere 3.OnComponentBeginOverlap` OtherActor))))))
          (message `/Game/damege_김세준/BPI_damagable.takedamage` (stale `self.Sphere 3.OnComponentBeginOverlap` OtherActor) (make `/Game/damege_김세준/s_damageinfo` 1.0 "NewEnumerator2" "NewEnumerator1" false false false false (`KismetMathLibrary.MakeVector` (* _returnvalue_x -1.0) (* _returnvalue_y -1.0) _returnvalue_z)))
          (`ActorComponent.K2_DestroyComponent` (`self.NewVar_3`)))))))

(event `self.Sphere 8.OnComponentBeginOverlap`
  (params (OverlappedComponent :type "PrimitiveComponent Object Reference") (OtherActor :type "Actor Object Reference") (OtherComp :type "PrimitiveComponent Object Reference") (OtherBodyIndex :type Integer) (bFromSweep :type Boolean) (SweepResult :type "HitResult Structure (by ref)"))
  (if (== OtherActor (`GameplayStatics.GetPlayerCharacter` 0))
    (goto _label_5)))

(event `self.Sphere 3.OnComponentBeginOverlap`
  (params (OverlappedComponent :type "PrimitiveComponent Object Reference") (OtherActor :type "Actor Object Reference") (OtherComp :type "PrimitiveComponent Object Reference") (OtherBodyIndex :type Integer) (bFromSweep :type Boolean) (SweepResult :type "HitResult Structure (by ref)"))
  (if (== OtherActor (`GameplayStatics.GetPlayerCharacter` 0))
    (goto _label_6)))

(event `시간제한 9`
  (`/Engine/EditorBlueprintResources/StandardMacros.DoOnce` false :!label _label_7
    (:`Completed`
      (`|ExecutionSequence`
        (:`then_0`
          (`GameplayStatics.SpawnSoundAtLocation` "/Game/Sound_AHJ/Cue/Monster/Phase/Cue_Monster_Stage_02_Phase_02_SFX.Cue_Monster_Stage_02_Phase_02_SFX" (0.0 0.0 0.0) (struct) 1.0 1.0 0.0 null null))
        (:`then_1`
          (`GameplayStatics.SpawnEmitterAtLocation` "/Game/StarterContent/Particles/P_Explosion1.P_Explosion1" (`SceneComponent.K2_GetComponentLocation` (`self.Sphere 9`)) (struct) (5.0 5.0 5.0))
          (bind (_returnvalue_x _returnvalue_y _returnvalue_z) (`KismetMathLibrary.BreakVector` (`KismetMathLibrary.GetForwardVector` (`SceneComponent.K2_GetComponentRotation` (`Actor.RootComponent` (stale `self.Sphere 9.OnComponentBeginOverlap` OtherActor))))))
          (message `/Game/damege_김세준/BPI_damagable.takedamage` (stale `self.Sphere 9.OnComponentBeginOverlap` OtherActor) (make `/Game/damege_김세준/s_damageinfo` 1.0 "NewEnumerator2" "NewEnumerator1" false false false false (`KismetMathLibrary.MakeVector` (* _returnvalue_x -1.0) (* _returnvalue_y -1.0) _returnvalue_z)))
          (`ActorComponent.K2_DestroyComponent` (`self.NewVar_9`)))))))

(event `시간제한 4`
  (`/Engine/EditorBlueprintResources/StandardMacros.DoOnce` false :!label _label_8
    (:`Completed`
      (`|ExecutionSequence`
        (:`then_0`
          (`GameplayStatics.SpawnSoundAtLocation` "/Game/Sound_AHJ/Cue/Monster/Phase/Cue_Monster_Stage_02_Phase_02_SFX.Cue_Monster_Stage_02_Phase_02_SFX" (0.0 0.0 0.0) (struct) 1.0 1.0 0.0 null null))
        (:`then_1`
          (`GameplayStatics.SpawnEmitterAtLocation` "/Game/StarterContent/Particles/P_Explosion1.P_Explosion1" (`SceneComponent.K2_GetComponentLocation` (`self.Sphere 4`)) (struct) (5.0 5.0 5.0))
          (bind (_returnvalue_x _returnvalue_y _returnvalue_z) (`KismetMathLibrary.BreakVector` (`KismetMathLibrary.GetForwardVector` (`SceneComponent.K2_GetComponentRotation` (`Actor.RootComponent` (stale `self.Sphere 4.OnComponentBeginOverlap` OtherActor))))))
          (message `/Game/damege_김세준/BPI_damagable.takedamage` (stale `self.Sphere 4.OnComponentBeginOverlap` OtherActor) (make `/Game/damege_김세준/s_damageinfo` 1.0 "NewEnumerator2" "NewEnumerator1" false false false false (`KismetMathLibrary.MakeVector` (* _returnvalue_x -1.0) (* _returnvalue_y -1.0) _returnvalue_z)))
          (`ActorComponent.K2_DestroyComponent` (`self.NewVar_4`)))))))

(event `self.Sphere 9.OnComponentBeginOverlap`
  (params (OverlappedComponent :type "PrimitiveComponent Object Reference") (OtherActor :type "Actor Object Reference") (OtherComp :type "PrimitiveComponent Object Reference") (OtherBodyIndex :type Integer) (bFromSweep :type Boolean) (SweepResult :type "HitResult Structure (by ref)"))
  (if (== OtherActor (`GameplayStatics.GetPlayerCharacter` 0))
    (goto _label_7)))

(event `self.Sphere 4.OnComponentBeginOverlap`
  (params (OverlappedComponent :type "PrimitiveComponent Object Reference") (OtherActor :type "Actor Object Reference") (OtherComp :type "PrimitiveComponent Object Reference") (OtherBodyIndex :type Integer) (bFromSweep :type Boolean) (SweepResult :type "HitResult Structure (by ref)"))
  (if (== OtherActor (`GameplayStatics.GetPlayerCharacter` 0))
    (goto _label_8)))

(event `시간제한 10`
  (`/Engine/EditorBlueprintResources/StandardMacros.DoOnce` false :!label _label_9
    (:`Completed`
      (`|ExecutionSequence`
        (:`then_0`
          (`GameplayStatics.SpawnSoundAtLocation` "/Game/Sound_AHJ/Cue/Monster/Phase/Cue_Monster_Stage_02_Phase_02_SFX.Cue_Monster_Stage_02_Phase_02_SFX" (0.0 0.0 0.0) (struct) 1.0 1.0 0.0 null null))
        (:`then_1`
          (`GameplayStatics.SpawnEmitterAtLocation` "/Game/StarterContent/Particles/P_Explosion1.P_Explosion1" (`SceneComponent.K2_GetComponentLocation` (`self.Sphere 10`)) (struct) (5.0 5.0 5.0))
          (bind (_returnvalue_x _returnvalue_y _returnvalue_z) (`KismetMathLibrary.BreakVector` (`KismetMathLibrary.GetForwardVector` (`SceneComponent.K2_GetComponentRotation` (`Actor.RootComponent` (stale `self.Sphere 10.OnComponentBeginOverlap` OtherActor))))))
          (message `/Game/damege_김세준/BPI_damagable.takedamage` (stale `self.Sphere 10.OnComponentBeginOverlap` OtherActor) (make `/Game/damege_김세준/s_damageinfo` 1.0 "NewEnumerator2" "NewEnumerator1" false false false false (`KismetMathLibrary.MakeVector` (* _returnvalue_x -1.0) (* _returnvalue_y -1.0) _returnvalue_z)))
          (`ActorComponent.K2_DestroyComponent` (`self.NewVar_10`)))))))

(event `시간제한 5`
  (`/Engine/EditorBlueprintResources/StandardMacros.DoOnce` false :!label _label_10
    (:`Completed`
      (`|ExecutionSequence`
        (:`then_0`
          (`GameplayStatics.SpawnSoundAtLocation` "/Game/Sound_AHJ/Cue/Monster/Phase/Cue_Monster_Stage_02_Phase_02_SFX.Cue_Monster_Stage_02_Phase_02_SFX" (0.0 0.0 0.0) (struct) 1.0 1.0 0.0 null null))
        (:`then_1`
          (`GameplayStatics.SpawnEmitterAtLocation` "/Game/StarterContent/Particles/P_Explosion1.P_Explosion1" (`SceneComponent.K2_GetComponentLocation` (`self.Sphere 5`)) (struct) (5.0 5.0 5.0))
          (bind (_returnvalue_x _returnvalue_y _returnvalue_z) (`KismetMathLibrary.BreakVector` (`KismetMathLibrary.GetForwardVector` (`SceneComponent.K2_GetComponentRotation` (`Actor.RootComponent` (stale `self.Sphere 5.OnComponentBeginOverlap` OtherActor))))))
          (message `/Game/damege_김세준/BPI_damagable.takedamage` (stale `self.Sphere 5.OnComponentBeginOverlap` OtherActor) (make `/Game/damege_김세준/s_damageinfo` 1.0 "NewEnumerator2" "NewEnumerator1" false false false false (`KismetMathLibrary.MakeVector` (* _returnvalue_x -1.0) (* _returnvalue_y -1.0) _returnvalue_z)))
          (`ActorComponent.K2_DestroyComponent` (`self.NewVar_5`)))))))

(event `self.Sphere 10.OnComponentBeginOverlap`
  (params (OverlappedComponent :type "PrimitiveComponent Object Reference") (OtherActor :type "Actor Object Reference") (OtherComp :type "PrimitiveComponent Object Reference") (OtherBodyIndex :type Integer) (bFromSweep :type Boolean) (SweepResult :type "HitResult Structure (by ref)"))
  (if (== OtherActor (`GameplayStatics.GetPlayerCharacter` 0))
    (goto _label_9)))

(event `self.Sphere 5.OnComponentBeginOverlap`
  (params (OverlappedComponent :type "PrimitiveComponent Object Reference") (OtherActor :type "Actor Object Reference") (OtherComp :type "PrimitiveComponent Object Reference") (OtherBodyIndex :type Integer) (bFromSweep :type Boolean) (SweepResult :type "HitResult Structure (by ref)"))
  (if (== OtherActor (`GameplayStatics.GetPlayerCharacter` 0))
    (goto _label_10)))

(fn `UserConstructionScript`)