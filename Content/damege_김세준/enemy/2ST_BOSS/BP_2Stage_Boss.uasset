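; Stage 2 boss enemy with health-based attack phases, an HP widget, intro montage, boss music and death sequence.
; Random montages form combos or drop water mines above half health, then switch to single attacks and an extending chain attack.
; Montage notifies bound timer-driven weapon sphere traces that stop after one damaging hit.
; BPCDamageSystem handles incoming damage, with responses for player hits, special-weapon stuns, knockback and a timed stun window.
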(event `attack_montage`
  (bind _returnvalue (`KismetMathLibrary.RandomInteger` 99))
  (bind _returnvalue_2 (`KismetMathLibrary.RandomInteger` 99))
  ;[1 1 1] 공격 모션 불러오기
  (set `self.IS ATTACKING` true)
  (set `CharacterMovementComponent.bAllowPhysicsRotationDuringAnimRootMotion` true (`self.CharacterMovement`))
  (if (`self.deathboleon`)
    _
    (elif (> (/ (`self.current Helth`) (`self.max Helth`)) 0.5)
      ;;[1 1 1] 1페이즈 패턴
      (if (>= _returnvalue_2 79)
        (set `self.공격 모션` "/Game/damege_김세준/enemy/2ST_BOSS/2st_Boss_montage/240107_anim_combo03_01_KSJ_Montage.240107_anim_combo03_01_KSJ_Montage")
        (`|PlayMontage` (`self.Mesh`) (`self.공격 모션`) (`self.공격 모션 배속`) :!label _label
          (:`OnCompleted`
            (`self.On attack end` :!label _label_2)
            (set `self.IS ATTACKING` false))
          (:`OnInterrupted`
            (goto _label_2))
          (:`OnNotifyBegin`
            (`self.공격` :!label _label_3)
            (set `CharacterMovementComponent.bAllowPhysicsRotationDuringAnimRootMotion` false (`self.CharacterMovement`)))
          (:`OnNotifyEnd`
            (`KismetSystemLibrary.K2_ClearAndInvalidateTimerHandle` (`self.무기 휘두르기`) :!label _label_4)
            (bind _returnvalue_3 (`GameplayStatics.GetActorOfClass` "/Game/damege_김세준/Player/BP_player_KSJ.BP_player_KSJ_C"))
            (if (not (`SceneComponent.bHiddenInGame` (`/Game/damege_김세준/Player/BP_player_KSJ.TextRender` _returnvalue_3)))
              (`/Game/damege_김세준/Player/BP_player_KSJ.알림 제거_Event` _returnvalue_3))))
        (elif (>= _returnvalue_2 59)
          (set `self.공격 모션` "/Game/damege_김세준/enemy/2ST_BOSS/2st_Boss_montage/240107_anim_combo03_01_KSJ_Montage.240107_anim_combo03_01_KSJ_Montage")
          (`|PlayMontage` (`self.Mesh`) (`self.공격 모션`) (`self.공격 모션 배속`)
            (:`OnCompleted`
              (set `self.공격 모션` "/Game/damege_김세준/enemy/2ST_BOSS/2st_Boss_montage/240107_anim_combo03_02_KSJ_Montage.240107_anim_combo03_02_KSJ_Montage")
              (goto _label))
            (:`OnInterrupted`
              (goto _label_2))
            (:`OnNotifyBegin`
              (goto _label_3))
            (:`OnNotifyEnd`
              (goto _label_2)))
          (elif (>= _returnvalue_2 39)
            (set `self.공격 모션` "/Game/damege_김세준/enemy/2ST_BOSS/2st_Boss_montage/240107_anim_combo03_01_KSJ_Montage.240107_anim_combo03_01_KSJ_Montage")
            (`|PlayMontage` (`self.Mesh`) (`self.공격 모션`) (`self.공격 모션 배속`)
              (:`OnCompleted`
                (set `self.공격 모션` "/Game/damege_김세준/enemy/2ST_BOSS/2st_Boss_montage/240107_anim_combo03_02_KSJ_Montage.240107_anim_combo03_02_KSJ_Montage")
                (`|PlayMontage` (`self.Mesh`) (`self.공격 모션`) (`self.공격 모션 배속`)
                  (:`OnCompleted`
                    (set `self.공격 모션` "/Game/damege_김세준/enemy/2ST_BOSS/2st_Boss_montage/240107_anim_combo03_03_KSJ_Montage.240107_anim_combo03_03_KSJ_Montage")
                    (goto _label))
                  (:`OnInterrupted`
                    (goto _label_2))
                  (:`OnNotifyBegin`
                    (goto _label_3))
                  (:`OnNotifyEnd`
                    (goto _label_2))))
              (:`OnInterrupted`
                (goto _label_2))
              (:`OnNotifyBegin`
                (goto _label_3))
              (:`OnNotifyEnd`
                (goto _label_2)))
            (elif (>= _returnvalue_2 29)
              (set `self.공격 모션` "/Game/damege_김세준/enemy/2ST_BOSS/2st_Boss_montage/240107_anim_combo03_KSJ_Montage.240107_anim_combo03_KSJ_Montage")
              (goto _label)
              (elif (>= _returnvalue_2 24)
                (set `self.공격 모션` "/Game/damege_김세준/enemy/2ST_BOSS/2st_Boss_montage/240107_anim_combo02_KSJ_Montage.240107_anim_combo02_KSJ_Montage")
                (goto _label)
                (elif (>= _returnvalue_2 19)
                  (set `self.공격 모션` "/Game/damege_김세준/enemy/2ST_BOSS/2st_Boss_montage/240107_anim_combo01_KSJ_Montage.240107_anim_combo01_KSJ_Montage")
                  (goto _label)
                  (else
                    (set `self.공격 모션` "/Game/damege_김세준/enemy/2ST_BOSS/2st_Boss_montage/240107_anim_combo01_03_KSJ_Montage.240107_anim_combo01_03_KSJ_Montage")
                    (`|PlayMontage` (`self.Mesh`) (`self.공격 모션`) (`self.공격 모션 배속`)
                      (:`OnCompleted`
                        (goto _label_2))
                      (:`OnInterrupted`
                        (goto _label_2))
                      (:`OnNotifyBegin`
                        (goto _label_3))
                      (:`OnNotifyEnd`
                        (`|SpawnActorFromClass` "/Game/damege_김세준/enemy/2ST_BOSS/BP_물지뢰.BP_물지뢰_C" (`SceneComponent.K2_GetComponentToWorld` (`self.Box`)) "Undefined" "MultiplyWithRoot" null null)
                        (goto _label_4))))))))))
      (else
        ;;[1 1 1] 2페이즈 패턴
        (if (>= _returnvalue 79)
          (set `self.공격 모션` "/Game/damege_김세준/enemy/2ST_BOSS/2st_Boss_montage/240107_anim_combo01_KSJ_Montage.240107_anim_combo01_KSJ_Montage")
          (`|PlayMontage` (`self.Mesh`) (`self.공격 모션`) 1.2 :!label _label_5
            (:`OnCompleted`
              (`self.On attack end` :!label _label_6)
              (set `self.IS ATTACKING` false))
            (:`OnInterrupted`
              (goto _label_6))
            (:`OnNotifyBegin`
              (`self.공격` :!label _label_7)
              (set `CharacterMovementComponent.bAllowPhysicsRotationDuringAnimRootMotion` false (`self.CharacterMovement`)))
            (:`OnNotifyEnd`
              (`KismetSystemLibrary.K2_ClearAndInvalidateTimerHandle` (`self.무기 휘두르기`) :!label _label_8)
              (bind _returnvalue_4 (`GameplayStatics.GetActorOfClass` "/Game/damege_김세준/Player/BP_player_KSJ.BP_player_KSJ_C"))
              (if (not (`SceneComponent.bHiddenInGame` (`/Game/damege_김세준/Player/BP_player_KSJ.TextRender` _returnvalue_4)))
                (`/Game/damege_김세준/Player/BP_player_KSJ.알림 제거_Event` _returnvalue_4))))
          (elif (>= _returnvalue 59)
            (set `self.공격 모션` "/Game/damege_김세준/enemy/2ST_BOSS/2st_Boss_montage/240107_anim_combo02_KSJ_Montage.240107_anim_combo02_KSJ_Montage")
            (goto _label_5)
            (elif (>= _returnvalue 39)
              (set `self.공격 모션` "/Game/damege_김세준/enemy/2ST_BOSS/2st_Boss_montage/240107_anim_combo03_KSJ_Montage.240107_anim_combo03_KSJ_Montage")
              (goto _label_5)
              (elif (>= _returnvalue 19)
                (set `self.공격 모션` "/Game/damege_김세준/enemy/2ST_BOSS/2st_Boss_montage/240107_anim_combo01_03_KSJ_Montage.240107_anim_combo01_03_KSJ_Montage")
                (goto _label_5)
                (else
                  (set `self.공격 모션` "/Game/damege_김세준/enemy/2ST_BOSS/2st_Boss_montage/240107_anim_atk_06_KSJ_Montage.240107_anim_atk_06_KSJ_Montage")
                  (set `self.사슬 공격` true)
                  (`|PlayMontage` (`self.Mesh`) (`self.공격 모션`) 0.5
                    (:`then`
                      (`SceneComponent.SetHiddenInGame` (`self.Main_weapon`) true false)
                      (`SceneComponent.SetHiddenInGame` (`self.S_Wall_Mounted_Chain_uiziegbdw_lod5`) false false)
                      (`SceneComponent.SetHiddenInGame` (`self.sub_weapon`) false false)
                      (bind _returnvalue_5 (`KismetSystemLibrary.K2_SetTimerDelegate` (delegate `체인 길어지기`) 0.01 true))
                      (set `self.사슬 길이 늘림` _returnvalue_5))
                    (:`OnCompleted`
                      (goto _label_6))
                    (:`OnInterrupted`
                      (goto _label_6))
                    (:`OnNotifyBegin`
                      (goto _label_7))
                    (:`OnNotifyEnd`
                      (goto _label_8))))))))))))

(event `Damageresponse`
  (params (Damageresponse :type "/Game/damege_김세준/E_DamageResponse Enum" :default "NewEnumerator0") (`대미지` :type "Float (double-precision)") (NewParam :type "Vector Structure") (NewParam2 :type "Rotator Structure") (NewParam3 :type "/Game/damege_김세준/E_damage_type Enum" :default "NewEnumerator0"))
  (bind (_returnvalue_x _returnvalue_y _returnvalue_z) (`KismetMathLibrary.BreakVector` (* NewParam 1200.0)))
  ;[1 1 1] 대미지 수신 노드
  (switch `/Game/damege_김세준/E_damage_type` NewParam3
    (:`NewEnumerator1`
      (set `self.대미지` `대미지`)
      (switch `/Game/damege_김세준/E_DamageResponse` Damageresponse
        (:`NewEnumerator1`
          (if (not (`self.무적 버프`))
            (if (`self.IS ATTACKING`)
              (bind _returnvalue (`GameplayStatics.GetActorOfClass` "/Game/damege_김세준/Player/BP_player_KSJ.BP_player_KSJ_C"))
              (`/Game/damege_김세준/Player/BP_player_KSJ.필살기 게이지 충전_Event` _returnvalue))
            (`AISense_Damage.ReportDamageEvent` self (`GameplayStatics.GetPlayerCharacter` 0) 1.0 :!label _label_9)
            (`KismetSystemLibrary.PrintString` (`|GetEnumeratorNameAsString` Damageresponse))
            (if (not (`self.deathboleon`))
              (bind _output_get (set `self.current Helth` (`KismetMathLibrary.FClamp` (- (`self.current Helth`) (`self.대미지`)) 0.0 (`self.max Helth`))))
              (`/Game/damege_김세준/enemy/2ST_BOSS/WB_2stBoss_HP.Update Helth Ui` (stale `플레이어 발견 시` _returnvalue) _output_get (`self.max Helth`))
              (if (>= 0.0 (`self.current Helth`))
                (`self.On attack end`)
                (set `self.deathboleon` true)
                (`self.dead`)))))
        (:`NewEnumerator2`
          (`KismetSystemLibrary.K2_ClearAndInvalidateTimerHandle` (`self.앞잡 타이머`))
          (set `self.앞잡 계산기` 0.0))
        (:`NewEnumerator3`
          (goto _label_9))
        (:`NewEnumerator4`
          (`|ExecutionSequence`
            (:`then_0`
              (set `self.넉백` true)
              (`self.LaunchCharacter` (`KismetMathLibrary.MakeVector` _returnvalue_x _returnvalue_y _returnvalue_z))
              (`KismetSystemLibrary.Delay` 2.0)
              (set `self.IS stun` false)
              (`self.스턴 해제`)
              (`self.On attack end`)
              (set `PrimitiveComponent.bGenerateOverlapEvents` false (`self.Box`))
              (set `self.넉백` false))
            (:`then_1`
              (goto _label_9))))))
    (:`NewEnumerator3`
      (set `self.IS ATTACKING` false)
      (`self.StopAnimMontage` (`self.공격 모션`))
      (set `self.IS stun` true)
      (`GameplayStatics.PlaySoundAtLocation` "/Game/Sound_AHJ/Cue/Monster/GetHit/Cue_Monster_GetHit_Groggy_SFX.Cue_Monster_GetHit_Groggy_SFX" (0.0 0.0 0.0) (struct) 1.0 1.0 0.0 null null null null))
    (:`NewEnumerator4`
      (set `self.IS ATTACKING` false)
      (`self.StopAnimMontage` (`self.공격 모션`))
      (set `self.IS stun` true)
      (goto _label_9))))

(event `self.Box.OnComponentBeginOverlap`
  (params (OverlappedComponent :type "PrimitiveComponent Object Reference") (OtherActor :type "Actor Object Reference") (OtherComp :type "PrimitiveComponent Object Reference") (OtherBodyIndex :type Integer) (bFromSweep :type Boolean) (SweepResult :type "HitResult Structure (by ref)"))
  ;[1 1 1] 앞잡 노드
  (message `/Game/damege_김세준/BPI_damagable.takedamage` OtherActor (make `/Game/damege_김세준/s_damageinfo` 1.0 "NewEnumerator2" "NewEnumerator3" false false false false (`SceneComponent.K2_GetComponentLocation` (`self.Box`)) (`KismetMathLibrary.Conv_VectorToRotator` (* (`SceneComponent.GetForwardVector` (`self.CapsuleComponent`)) -1.0)))))

(event `스턴`
  ;[1 1 1] 앞잡 노드
  (set `PrimitiveComponent.bGenerateOverlapEvents` true (`self.Box`))
  (bind _returnvalue (`KismetSystemLibrary.K2_SetTimerDelegate` (delegate `앞잡 카운트다운`) 1.0 true))
  (set `self.앞잡 타이머` _returnvalue))

(event `앞잡 카운트다운`
  ;[1 1 1] 앞잡 노드
  (bind _output_get (set `self.앞잡 계산기` (+ (`self.앞잡 계산기`) 1.0)))
  (if (== _output_get 3.0)
    (`self.스턴 해제`)
    (`self.On attack end`)
    (set `self.IS stun` false)
    (set `PrimitiveComponent.bGenerateOverlapEvents` false (`self.Box`))))

(event `체력충전`
  ;[1 1 1] UI 업데이트
  (bind _output_get (set `self.current Helth` (`self.max Helth`)))
  (`/Game/damege_김세준/enemy/2ST_BOSS/WB_2stBoss_HP.Update Helth Ui` (stale `플레이어 발견 시` _returnvalue) _output_get (`self.max Helth`)))

(event `플레이어 발견 시`
  ;[1 1 1] 플레이어 발견시 위젯 생성
  (`|ExecutionSequence`
    (:`then_0`
      (bind _returnvalue (`|CreateWidget` "/Game/damege_김세준/enemy/2ST_BOSS/WB_2stBoss_HP.WB_2stBoss_HP_C" (`GameplayStatics.GetPlayerController` 0) self))
      (`UserWidget.AddToViewport` _returnvalue 0)
      (`self.체력충전`)
      (`/Engine/EditorBlueprintResources/StandardMacros.DoOnce` false
        (:`Completed`
          (`|PlayMontage` (`self.Mesh`) "/Game/damege_김세준/enemy/2ST_BOSS/CaveTrollLight/Animations/Cave_troll_danger_attack_0_Montage.Cave_troll_danger_attack_0_Montage"
            (:`then`
              (`self.보스전 시작`))
            (:`OnCompleted`
              (set `self.draw waepon` true))))))
    (:`then_1`
      (`/Engine/EditorBlueprintResources/StandardMacros.DoOnce` false
        (:`Completed`
          (bind _returnvalue_2 (`GameplayStatics.GetActorOfClass` "/Game/damege_김세준/Player/BP_player_KSJ.BP_player_KSJ_C"))
          (`/Game/damege_김세준/Player/BP_player_KSJ.Stage 2보스 BGM_Event` _returnvalue_2))))))

(event `공격`
  ;[1 1 1] 공격 로직
  (bind _returnvalue (`KismetSystemLibrary.K2_SetTimerDelegate` (delegate `대미지 처리`) 0.01 true))
  (set `self.무기 휘두르기` _returnvalue)
  (bind _returnvalue_2 (`GameplayStatics.GetActorOfClass` "/Game/damege_김세준/Player/BP_player_KSJ.BP_player_KSJ_C"))
  (if (`SceneComponent.bHiddenInGame` (`/Game/damege_김세준/Player/BP_player_KSJ.TextRender` _returnvalue_2))
    (`/Game/damege_김세준/Player/BP_player_KSJ.딜레이캐치 알림_Event` _returnvalue_2)))

(event `dead`
  ;[1 1 1] 몹 사망 이벤트
  (`/Engine/EditorBlueprintResources/StandardMacros.DoOnce` false
    (:`Completed`
      (`self.StopAnimMontage` (`self.공격 모션`))
      (`SkeletalMeshComponent.PlayAnimation` (`self.Mesh`) "/Game/animcore/2Handed_HammerSet/Animation/dead01_H_wjm.dead01_H_wjm" false)
      (`GameplayStatics.PlaySoundAtLocation` "/Game/Sound_AHJ/Cue/Monster/Cue_Boss_Monster_Die_SFX.Cue_Boss_Monster_Die_SFX" (0.0 0.0 0.0) (struct) 1.0 1.0 0.0 null null null null)
      (`KismetSystemLibrary.Delay` 5.0)
      (`/Engine/EditorBlueprintResources/StandardMacros.DoOnce` false
        (:`Completed`
          (`ActorComponent.K2_DestroyComponent` (`self.enemy HP bar`))
          (`KismetSystemLibrary.Delay` 5.0)
          (`self.K2_DestroyActor`))))))

(event `대미지 처리`
  (bind _main_weapon (`self.Main_weapon`))
  ;[1 1 1] 공격 로직
  (if (`self.deathboleon`)
    _
    (elif (not (`self.사슬 공격`))
      (bind (_outhit _returnvalue) (`KismetSystemLibrary.SphereTraceSingle` :`Start` (`SceneComponent.GetSocketLocation` _main_weapon "start") :`End` (`SceneComponent.GetSocketLocation` _main_weapon "end") :`Radius` 150.0 :`TraceChannel` "TraceTypeQuery1" :`DrawTime` 0.0))
      (if _returnvalue
        (bind (_bblockinghit _binitialoverlap _time _distance _location _impactpoint _normal _impactnormal _physmat _hitactor) (`GameplayStatics.BreakHitResult` _outhit))
        (bind (_wasdamaged `_대미지_입력값`) (message `/Game/damege_김세준/BPI_damagable.takedamage` _hitactor (make `/Game/damege_김세준/s_damageinfo` 1.0 "NewEnumerator2" "NewEnumerator1" false false false false (`KismetMathLibrary.GetForwardVector` (`SceneComponent.K2_GetComponentRotation` (`self.CapsuleComponent`))))))
        (if _wasdamaged
          (`KismetSystemLibrary.PrintString` (`KismetStringLibrary.Conv_DoubleToString` `_대미지_입력값`))
          (`GameplayStatics.SpawnEmitterAtLocation` "/Game/StarterContent/Particles/P_Explosion.P_Explosion" _location)
          (`self.다단히트 금지`)))
      (else
        (bind (_outhit_2 _returnvalue_2) (`KismetSystemLibrary.SphereTraceSingle` :`Start` (`SceneComponent.GetSocketLocation` (`self.S_Wall_Mounted_Chain_uiziegbdw_lod5`) "start") :`End` (`SceneComponent.GetSocketLocation` (`self.sub_weapon`) "end") :`Radius` 150.0 :`TraceChannel` "TraceTypeQuery1" :`DrawTime` 0.0))
        (if _returnvalue_2
          (bind (_bblockinghit_2 _binitialoverlap_2 _time_2 _distance_2 _location_2 _impactpoint_2 _normal_2 _impactnormal_2 _physmat_2 _hitactor_2) (`GameplayStatics.BreakHitResult` _outhit_2))
          (bind (_wasdamaged_2 `_대미지_입력값_2`) (message `/Game/damege_김세준/BPI_damagable.takedamage` _hitactor_2 (make `/Game/damege_김세준/s_damageinfo` 1.0 "NewEnumerator2" "NewEnumerator1" false false false false (`KismetMathLibrary.GetForwardVector` (`SceneComponent.K2_GetComponentRotation` (`self.CapsuleComponent`))))))
          (if _wasdamaged_2
            (`KismetSystemLibrary.PrintString` (`KismetStringLibrary.Conv_DoubleToString` `_대미지_입력값_2`))
            (`GameplayStatics.SpawnEmitterAtLocation` "/Game/StarterContent/Particles/P_Explosion.P_Explosion" _location_2)
            (`self.다단히트 금지`)))))))

(event `다단히트 금지`
  ;[1 1 1] 공격 로직
  (`KismetSystemLibrary.K2_ClearAndInvalidateTimerHandle` (`self.무기 휘두르기`)))

(event `체인 길어지기`
  (bind _s_wall_mounted_chain_uiziegbdw_lod5 (`self.S_Wall_Mounted_Chain_uiziegbdw_lod5`))
  (bind (_relativescale3d_x _relativescale3d_y _relativescale3d_z) (`KismetMathLibrary.BreakVector` (`SceneComponent.RelativeScale3D` _s_wall_mounted_chain_uiziegbdw_lod5)))
  ;[1 1 1] 공격 모션 불러오기
  ;;[1 1 1] 2페이즈 패턴
  (bind _output_get (set `self.Relative Scale 3D X` (+ _relativescale3d_x 0.02)))
  (`SceneComponent.SetRelativeScale3D` _s_wall_mounted_chain_uiziegbdw_lod5 (`KismetMathLibrary.MakeVector` _output_get _relativescale3d_y _relativescale3d_z))
  (if (>= (`self.Relative Scale 3D X`) 1.0)
    (`KismetSystemLibrary.K2_ClearAndInvalidateTimerHandle` (`self.사슬 길이 늘림`))
    (`KismetSystemLibrary.Delay` 1.0)
    (bind _returnvalue (`KismetSystemLibrary.K2_SetTimerDelegate` (delegate `체인이 줄어듬`) 0.01 true))
    (set `self.사슬 길이 줄임` _returnvalue)))

(event `체인이 줄어듬`
  (bind _s_wall_mounted_chain_uiziegbdw_lod5 (`self.S_Wall_Mounted_Chain_uiziegbdw_lod5`))
  (bind (_relativescale3d_x _relativescale3d_y _relativescale3d_z) (`KismetMathLibrary.BreakVector` (`SceneComponent.RelativeScale3D` _s_wall_mounted_chain_uiziegbdw_lod5)))
  ;[1 1 1] 공격 모션 불러오기
  ;;[1 1 1] 2페이즈 패턴
  (bind _output_get (set `self.Relative Scale 3D X` (- _relativescale3d_x 0.02)))
  (`SceneComponent.SetRelativeScale3D` _s_wall_mounted_chain_uiziegbdw_lod5 (`KismetMathLibrary.MakeVector` _output_get _relativescale3d_y _relativescale3d_z))
  (if (<= (`self.Relative Scale 3D X`) 0.1)
    (`KismetSystemLibrary.K2_ClearAndInvalidateTimerHandle` (`self.사슬 길이 줄임`))
    (`SceneComponent.SetHiddenInGame` (`self.Main_weapon`) false false)
    (`SceneComponent.SetHiddenInGame` (`self.S_Wall_Mounted_Chain_uiziegbdw_lod5`) true false)
    (`SceneComponent.SetHiddenInGame` (`self.sub_weapon`) true false)
    (set `self.사슬 공격` false)))

(fn `gatmaxhealth`
  (returns (maxhealth :type "Float (double-precision)"))
  (return (`self.max Helth`)))

(fn `get idial range`
  (returns (`attack radius` :type "Float (double-precision)") (`defend radius` :type "Float (double-precision)"))
  (return 1000.0 1100.0))

(fn `get patroll route`
  (returns (`patroll route` :type "/Game/damege_김세준/enemy/AI_Base/patrol_rap Object Reference"))
  (return (`self.patrollroute`)))

(fn `getcurrenthealth`
  (returns (health :type "Float (double-precision)"))
  (return (`self.current Helth`)))

(fn `heal`
  (params (amount :type "Float (double-precision)"))
  (returns (newhealth :type "Float (double-precision)"))
  (bind _newhealth (`/Game/damege_김세준/BPC_damageSystem.heal` (`self.BPC_damageSystem`) amount))
  (return _newhealth))

(fn `set movement speed`
  (params (speed :type "/Game/damege_김세준/enemy/AI_Base/Enums/E_movementspeed Enum" :default "NewEnumerator0"))
  (returns (`speed velue` :type "Float (double-precision)"))
  (bind _output_get (set `CharacterMovementComponent.MaxWalkSpeed` (select `/Game/damege_김세준/enemy/AI_Base/Enums/E_movementspeed` speed :`NewEnumerator1` 100.0 :`NewEnumerator2` 300.0 :`NewEnumerator3` 500.0 :!type "Float (single-precision)") (`self.CharacterMovement`)))
  (return _output_get))

(fn `takedamage`
  (params (Damageinfo :type "/Game/damege_김세준/s_damageinfo Structure"))
  (returns (WasDamaged :type Boolean) (`대미지 입력값` :type "Float (double-precision)"))
  (bind (_was_damaged `_대미지_입력값`) (`/Game/damege_김세준/BPC_damageSystem.TakeDamge` (`self.BPC_damageSystem`) Damageinfo (`self.current Helth`) (`self.max Helth`) (`self.deathboleon`)))
  (return _was_damaged `_대미지_입력값`))

(fn `UserConstructionScript`
  (bind _bpc_damagesystem (`self.BPC_damageSystem`))
  (add `/Game/damege_김세준/BPC_damageSystem.Ondeath` _bpc_damagesystem (`|CreateDelegate` :!event `dead`))
  (add `/Game/damege_김세준/BPC_damageSystem.Ondamageresponse` _bpc_damagesystem (`|CreateDelegate` :!event `Damageresponse`)))