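; Actor component for a damage system that tracks health, death, invincibility and blocking state.
; Heal adds health clamped to the maximum while alive.
; TakeDamge stores the passed-in death flag and broadcasts the damage info through a damage response dispatcher, without reducing Health itself.
; A separate canbedamaged macro routes hits to damage, block or no damage, with per-hit overrides for invincibility and blockability.
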(fn `heal`
  (params (amount :type "Float (double-precision)"))
  (returns (Newhealth :type "Float (double-precision)"))
  (if (not (`self.Isdead`))
    (bind _output_get (set `self.Health` (`KismetMathLibrary.FClamp` (+ amount (`self.Health`)) 0.0 (`self.MaxHealth`))))
    (return _output_get)))

(fn `TakeDamge`
  (params (Damageinfo :type "/Game/damege_김세준/s_damageinfo Structure") (`Current Health` :type "Float (double-precision) (by ref)") (`Max Health` :type "Float (double-precision) (by ref)") (`IS DEAD` :type "Boolean (by ref)"))
  (returns (`was damaged` :type Boolean) (`대미지 입력값` :type "Float (double-precision)"))
  (locals (NewLocalVar :type "/Game/damege_김세준/E_damage_type Enum" :default "NewEnumerator0"))
  (bind (_amount _damagetype _damageresponse _shoulddamageinvincible _canbeblocked _canbeparried _shouldforceinterrupt _whohit _whereitsface) (break `/Game/damege_김세준/s_damageinfo` Damageinfo))
  (set `self.Isdead` `IS DEAD`)
  (`self.Ondamageresponse` _damageresponse _amount _whohit _whereitsface _damagetype)
  (return true _amount))